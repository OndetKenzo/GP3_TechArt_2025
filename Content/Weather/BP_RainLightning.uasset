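; Weather actor that runs rain with recurring lightning strikes around the player.
; ToggleRain switches a Niagara rain effect that follows the player each tick and loops randomly delayed strikes, each briefly boosting post-process exposure as a flash.
; Strikes move the actor far ahead of the camera, yaw it toward the player, and animate plane materials through a timeline.
; SetRainDensity drives both height fog and rain density.
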(event Custom|Strike
  (bind _lightning_plane (Variables|Default|GetLightning_plane))
  ;[0.15 0.15 0.15 0.5] Lightning Behaviour
  (CallFunction|Locateat)
  (bind _y (Timeline|LigntningStrike PlayFromStart)
    (:Update
      (Rendering|Material|SetScalarParameterValueonMaterials _lightning_plane "Y" _y)
      (Rendering|Material|SetScalarParameterValueonMaterials _lightning_plane "emission" (* (+ _y 1.0) 5e+01)))))

(event Custom|LocateAt
  (bind _returnvalue (Math|Random|RandomFloatinRange -8e+04 8e+04))
  (bind _returnvalue_2 (Game|GetPlayerCharacter 0))
  (bind _returnvalue_3 (Math|Random|RandomFloatinRange 8e+04 1e+05))
  (bind _returnvalue_4 (Game|GetPlayerController 0))
  (bind _returnvalue_5 (Transformation|GetActorLocation _returnvalue_2))
  (bind _returnvalue_6 (Pawn|GetControlRotation _returnvalue_4 :!class /Script/Engine.Controller))
  (bind _returnvalue_7 (Math|Vector|GetRightVector _returnvalue_6))
  (bind _returnvalue_8 (Math|Vector|GetForwardVector _returnvalue_6))
  (bind _returnvalue_9 (* _returnvalue_7 _returnvalue))
  (bind _returnvalue_10 (* _returnvalue_8 _returnvalue_3))
  (bind _returnvalue_11 (+ _returnvalue_10 _returnvalue_9 _returnvalue_5))
  ;[0.15 0.15 0.15 0.5] Lightning Behaviour
  (Transformation|SetActorLocationAndRotation (Math|Vector|MakeVector (.x _returnvalue_11) (.y _returnvalue_11) 2.5e+04) (Math|Rotator|MakeRotator 0.0 0.0 (.yaw (Math|Rotator|FindLookatRotation (Math|Vector|MakeVector (.x _returnvalue_11) (.y _returnvalue_11) (.z _returnvalue_11)) _returnvalue_5)))))

(event Custom|ToggleRain
  (params (Enable/Disable :type Boolean))
  (bind _pp_volume (Variables|Default|GetPP_Volume))
  (bind _ns_raindrop (Variables|Default|GetNS_RainDrop))
  ;[0.15 0.15 0.15 0.5] Rain behaviour
  (if Enable/Disable
    (Variables|Default|SetRainEnabled true)
    (Components|Activation|Activate _ns_raindrop false)
    (Transformation|DetachFromComponent (Variables|Default|GetNS_RainDrop) "KeepRelative" "KeepRelative" "KeepRelative" true)
    (Utilities|IsValid (Variables|Default|GetPP_Volume)
      (:Is%20Valid
        (if (Variables|Default|GetRainEnabled)
          (Utilities|FlowControl|Delay (Math|Random|RandomFloatinRange 2.0 6.0) :!label _label)
          (if (Variables|Default|GetRainEnabled)
            (CallFunction|Strike)
            (Utilities|FlowControl|Delay 0.2)
            (bind _output_get (Variables|Default|SetOriginalExposure%20Compensation (Utilities|Struct|BreakPostProcessSettings (Variables|/Script/Engine.PostProcessVolume|GetSettings _pp_volume))))
            (Variables|/Script/Engine.PostProcessVolume|SetSettings _pp_volume (Utilities|Struct|MakePostProcessSettings "AEM_Manual" (+ _output_get 1.5)))
            (Utilities|FlowControl|Delay 0.2)
            (Variables|/Script/Engine.PostProcessVolume|SetSettings _pp_volume (Utilities|Struct|MakePostProcessSettings "AEM_Manual" _output_get))
            (goto _label))))
      (:Is%20Not%20Valid
        (|PostProcessVolumeCheck
          (:OutputPin
            (goto _label))
          (:No%20Post%20Process%20Volume
            (Development|PrintString "No Post Process Volume")))))
    (else
      (Components|Activation|Deactivate _ns_raindrop)
      (Variables|Default|SetRainEnabled false))))

(event EventBeginPlay
  (bind _heighfog (Variables|Default|GetHeighFog)
    (:then
      (Variables|Default|SetDefaultFog%20Density (Variables|/Script/Engine.ExponentialHeightFogComponent|GetFogDensity (Variables|/Script/Engine.ExponentialHeightFog|GetComponent _heighfog))))
    (:else)))

(event Collision|EventActorBeginOverlap
  (params (OtherActor :type Actor%20Object%20Reference)))

(event EventTick
  (params (DeltaSeconds :type Float%20%28single-precision%29))
  ;[0.15 0.15 0.15 0.5] Rain follow player
  (Transformation|SetWorldLocation (Variables|Default|GetNS_RainDrop) (+ (Transformation|GetActorLocation (Game|GetPlayerCharacter 0)) "0.000000,0.000000,1000.000000") false false))

(fn ConstructionScript)

(fn SetRainDensity
  (params (Density :type Float%20%28double-precision%29))
  (bind _heighfog (Variables|Default|GetHeighFog)
    (:then
      (Class|ExponentialHeightFogComponent|SetFogDensity (Variables|/Script/Engine.ExponentialHeightFog|GetComponent _heighfog) (Math|Float|Lerp (Variables|Default|GetDefaultFog%20Density) (Variables|Default|GetMaxRainFogDensity) Density))
      (Niagara|SetNiagaraVariable(Float) (Variables|Default|GetNS_RainDrop) "User.Density" Density))
    (:else)))