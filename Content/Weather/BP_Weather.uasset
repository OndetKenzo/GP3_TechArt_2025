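; Weather controller actor that toggles cloudy skies and rain through events.
; Cloud toggles set atmosphere targets, and Tick eases sky Rayleigh scattering, post-process exposure and volumetric cloud density toward them, disabling itself once exposure converges.
; Rain toggles swap the player's footstep sound and particle system and switch the rain effect.
; A reversible RainStrenght timeline drives rain density, prop wetness and moss material parameters, and a global wetness parameter collection.
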(event Custom|Start/StopRain
  (bind _player (Variables|Default|GetPlayer))
  (bind _audiocomponent (Variables|/Game/ThirdPerson/Blueprints/BP_ThirdPersonCharacter.BP_ThirdPersonCharacter_C|GetAudioComponent _player))
  ;[0.15 0.15 0.15 0.5] Toggle Rain
  (Variables|Default|GetIsRainning
    (:then
      (Variables|Default|SetIsRainning false)
      (Audio|Components|Audio|SetSound _audiocomponent "/Game/Sounds/BasicStepSound.BasicStepSound")
      (Variables|/Game/ThirdPerson/Blueprints/BP_ThirdPersonCharacter.BP_ThirdPersonCharacter_C|SetFootstepSystem _player "/Game/A_Surface_Footstep/Niagara_FX/ParticleSystems/PSN_Dirt_Surface.PSN_Dirt_Surface")
      (Default|ToggleRain (Variables|Default|GetRain) false)
      (bind _rain_level (Timeline|RainStrenght Reverse)
        (:Update
          (bind _returnvalue (Rendering|Material|CreateDynamicMaterialInstance (Variables|/Script/Engine.StaticMeshActor|GetStaticMeshComponent (Variables|Default|GetProps)) 0 "/Game/Materials/Instance/MI_Props_02.MI_Props_02" "None" :!class /Script/Engine.PrimitiveComponent))
          (Rendering|Material|SetScalarParameterValue _returnvalue "Moss_Amount" _rain_level :!class /Script/Engine.MaterialInstanceDynamic)
          (Rendering|Material|SetScalarParameterValue _returnvalue "Wetness" _rain_level :!class /Script/Engine.MaterialInstanceDynamic)
          (Rendering|Material|SetScalarParameterValue _returnvalue "RainDrops_Amount" _rain_level :!class /Script/Engine.MaterialInstanceDynamic)
          (Rendering|Material|SetScalarParameterValue _returnvalue "Moss_Hardness" _rain_level :!class /Script/Engine.MaterialInstanceDynamic)
          (Rendering|Material|SetScalarParameterValue _returnvalue "Moss_Dispersion" _rain_level :!class /Script/Engine.MaterialInstanceDynamic)
          (Rendering|Material|SetScalarParameterValue "/Game/Weather/Rain/MPC_Wetness.MPC_Wetness" "WetnessLevel" _rain_level :!class /Script/Engine.KismetMaterialLibrary)
          (Default|SetRainDensity (Variables|Default|GetRain) (* _rain_level 0.5)))))
    (:else
      (Variables|Default|SetIsRainning true)
      (Audio|Components|Audio|SetSound _audiocomponent "/Game/Sounds/RainStepSound.RainStepSound")
      (Variables|/Game/ThirdPerson/Blueprints/BP_ThirdPersonCharacter.BP_ThirdPersonCharacter_C|SetFootstepSystem _player "/Game/A_Surface_Footstep/Niagara_FX/ParticleSystems/PSN_WaterLight_Surface.PSN_WaterLight_Surface")
      (bind _rain (Variables|Default|GetRain)
        (:then
          (Default|ToggleRain _rain true)
          (Timeline|RainStrenght Play))
        (:else)))))

(event Custom|Start/Stop%20Cloud
  ;[0.15 0.15 0.15 0.5] Toggle Cloudy weather
  (Variables|Default|GetIsCloudy
    (:then
      (Variables|Default|SetIsCloudy false)
      (CallFunction|SetAtmosphereTargetParamters 1e+01 "(R=0.176471,G=0.407843,B=1.000000,A=1.000000)" "(R=0.502887,G=0.799103,B=0.502887,A=0.000000)"))
    (:else
      (Variables|Default|SetIsCloudy true)
      (CallFunction|SetAtmosphereTargetParamters 9.0 "(R=0.352941,G=0.368627,B=0.368627,A=1.000000)" (Math|Conversions|ToLinearColor(Float) (Math|Float|MakeLiteralFloat 0.1))))))

(event Custom|SetAtmosphereTargetParamters
  (params (Target%20Exposure%20Compensation :type Float%20%28single-precision%29) (Rayleigh%20Scattering :type Linear%20Color%20Structure) (Target%20Cloud%20Density :type Linear%20Color%20Structure))
  ;[0.15 0.15 0.15 0.5] Atmosphere
  (Variables|AtmosphereValues|SetTarget%20Cloud%20Density Target%20Cloud%20Density)
  (Variables|AtmosphereValues|SetTarget%20Exposure%20Compensation Target%20Exposure%20Compensation)
  (Variables|AtmosphereValues|SetTarget%20Rayleigh%20Scattering Rayleigh%20Scattering)
  (Actor|Tick|SetActorTickEnabled true))

(event EventBeginPlay
  (bind _returnvalue (Actor|GetActorOfClass "/Game/ThirdPerson/Blueprints/BP_ThirdPersonCharacter.BP_ThirdPersonCharacter_C"))
  (Variables|Default|SetPlayer _returnvalue))

(event Collision|EventActorBeginOverlap
  (params (OtherActor :type Actor%20Object%20Reference)))

(event EventTick
  (params (DeltaSeconds :type Float%20%28single-precision%29))
  (bind _returnvalue (Math|Float|MakeLiteralFloat 0.5))
  (bind _exposure_compensation (Variables|AtmosphereValues|GetExposure%20Compensation))
  (bind _target_exposure_compensation (Variables|AtmosphereValues|GetTarget%20Exposure%20Compensation))
  ;[0.15 0.15 0.15 0.5] Atmosphere
  (CallFunction|SetAtmosphere (Class|KismetMathLibrary|CInterpto (Variables|AtmosphereValues|GetRayleigh%20Scattering) (Variables|AtmosphereValues|GetTarget%20Rayleigh%20Scattering) DeltaSeconds _returnvalue) (Math|Interpolation|FInterptoConstant _exposure_compensation _target_exposure_compensation DeltaSeconds _returnvalue) (Class|KismetMathLibrary|CInterpto (Variables|AtmosphereValues|GetCloud%20Density) (Variables|AtmosphereValues|GetTarget%20Cloud%20Density) DeltaSeconds _returnvalue))
  (Actor|Tick|SetActorTickEnabled (not (Math|Float|NearlyEqual(Float) _exposure_compensation _target_exposure_compensation 0.05))))

(fn ConstructionScript)

(fn SetAtmosphere
  (params (Rayleigh%20Scattering :type Linear%20Color%20Structure) (Exposure%20Compensation :type Float%20%28single-precision%29) (Cloud%20Density :type Linear%20Color%20Structure))
  (Variables|AtmosphereValues|SetCloud%20Density Cloud%20Density)
  (Variables|AtmosphereValues|SetExposure%20Compensation Exposure%20Compensation)
  (Variables|AtmosphereValues|SetRayleigh%20Scattering Rayleigh%20Scattering)
  (bind _skyatmosphere (Variables|Default|GetSkyAtmosphere)
    (:then
      (Class|SkyAtmosphereComponent|SetRayleighScattering (Variables|/Script/Engine.SkyAtmosphere|GetSkyAtmosphereComponent _skyatmosphere) Rayleigh%20Scattering))
    (:else
      (Development|PrintString "Assign SkyAtmosphere")))
  (bind _postprocessvolume (Variables|Default|GetPostProcessVolume)
    (:then
      (Utilities|Struct|SetmembersinPostProcessSettings (Variables|/Script/Engine.PostProcessVolume|GetSettings _postprocessvolume) Exposure%20Compensation))
    (:else
      (Development|PrintString "Assign PostProcess volume")))
  (bind _volumetricclouds (Variables|Default|GetVolumetricClouds)
    (:then
      (Variables|Default|GetCloudMat
        (:then
          _)
        (:else
          (bind _returnvalue (Rendering|Material|CreateDynamicMaterialInstance "/Game/VolumetricClouds/MI_StormClouds.MI_StormClouds" "MClouds" "None" :!class /Script/Engine.KismetMaterialLibrary))
          (Variables|Default|SetCloudMat _returnvalue)))
      (Rendering|Material|SetMaterial (Variables|/Script/Engine.VolumetricCloud|GetVolumetricCloudComponent _volumetricclouds) (Variables|Default|GetCloudMat))
      (Rendering|Material|SetVectorParameterValue (Variables|Default|GetCloudMat) "Noise_Bias" Cloud%20Density :!class /Script/Engine.MaterialInstanceDynamic))
    (:else
      (Development|PrintString "Assign Volumetric Clouds"))))