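; Day/night cycle that rotates a directional light each tick, scaling its speed by NightLength while the sun is below the horizon.
; Light pitch drives sky material glow and opacity, and the opacity value's sign sets IsNight.
; Night calls the snow actor, shows auroras and activates a meteor shower; day turns auroras and meteor effects off.
; A DoOnce, reset during day, counts nights to trigger meteor rain every third night.
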(event Custom|MeteorRain
  (Utilities|FlowControl|DoOnce false
    (:Completed
      (Variables|Default|SetNightCount (+ (Variables|Default|GetNightCount) 1.0))
      (if (>= (Variables|Default|GetNightCount) 3.0)
        (Variables|Default|SetNightCount 0.0)
        (Components|Activation|Activate (Variables|/Script/Niagara.NiagaraActor|GetNiagaraComponent (Variables|Default|GetNS_MeteorRain)) false)))))

(event EventTick
  (params (DeltaSeconds :type Float%20%28single-precision%29))
  (bind _sunspeed (Variables|Default|GetSunSpeed))
  (bind _ns_meteorrain (Variables|Default|GetNS_MeteorRain))
  (bind _auroraborealis (Variables|Default|GetAuroraBorealis))
  (bind _opacityvalue (Variables|Default|GetOpacityValue))
  (bind _light (Variables|Default|GetLight))
  (bind _skymesh (Variables|Default|GetSkyMesh))
  (bind _nsmeteorshower (Variables|Default|GetNSMeteorShower))
  (bind _returnvalue (Transformation|GetActorRotation _light))
  (bind _rootcomponent (Variables|/Script/Engine.Actor|GetRootComponent _nsmeteorshower))
  (bind _niagaracomponent (Variables|/Script/Niagara.NiagaraActor|GetNiagaraComponent _ns_meteorrain))
  (bind _staticmeshcomponent (Variables|/Script/Engine.StaticMeshActor|GetStaticMeshComponent _skymesh))
  (bind _returnvalue_2 (/ (.pitch _returnvalue) 9e+01))
  (bind _returnvalue_3 (+ _returnvalue_2 0.1))
  (bind _returnvalue_4 (/ _returnvalue_3 2.0))
  (bind _returnvalue_5 (* _returnvalue_4 _opacityvalue))
  (Class|Actor|AddActorWorldRotation _light (Math|Rotator|MakeRotator 0.0 (* DeltaSeconds (Math|Float|SelectFloat _sunspeed (* _sunspeed (Variables|Default|GetNightLength)) (Math|Float|InRange(Float) (.pitch _returnvalue) -9e+01 0.0))) 0.0))
  (Rendering|Material|SetScalarParameterValueonMaterials _staticmeshcomponent "Glow Clank" (* _returnvalue_4 (Variables|Default|GetGlow%20Crank)))
  (Rendering|Material|SetScalarParameterValueonMaterials _staticmeshcomponent "Opacity multi" _returnvalue_5)
  (if (> _returnvalue_5 0.0)
    (Variables|Default|SetIsNight true)
    (Default|SnowFont (Variables|Default|GetBpSnow))
    (Components|Activation|Activate _rootcomponent false)
    (for _array_element _auroraborealis
      (Rendering|SetVisibility (Variables|/Script/Engine.Actor|GetRootComponent _array_element) true false)
      (CallFunction|MeteorRain)
      (Variables|Default|SetDayTime 0.0)
      (Variables|Default|SetDayTime 0.0))
    (else
      (Variables|Default|SetIsNight false)
      (Components|Activation|Deactivate _rootcomponent)
      (Components|Activation|Deactivate _niagaracomponent)
      (for _array_element_2 _auroraborealis
        (Rendering|SetVisibility (Variables|/Script/Engine.Actor|GetRootComponent _array_element_2) false false)
        (Utilities|FlowControl|DoOnce false) ; enters at Reset
      ))))

(fn ConstructionScript)