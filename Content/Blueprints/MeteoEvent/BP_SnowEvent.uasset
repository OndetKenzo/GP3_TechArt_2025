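; Snow weather event actor that toggles between snowfall and thaw, changing light, sky atmosphere, fog, Niagara snow and the player's footstep effects and sound.
; Nested timelines animate landscape ice, then house snow amount and hardness through material parameters, reversing on thaw.
; At night, snowfall still sets the snowing state and footsteps but skips visual changes and prints a warning.
; A DoOnce guards the thaw until the next snowfall.
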(event Custom|SnowFall
  (bind _player (Variables|Default|GetPlayer))
  (bind _floor (Variables|Default|GetFloor))
  (bind _skyatmosphere (Variables|Default|GetSkyAtmosphere))
  (bind _light (Variables|Default|GetLight))
  (bind _fog (Variables|Default|GetFog))
  (bind _component (Variables|/Script/Engine.ExponentialHeightFog|GetComponent _fog))
  (bind _skyatmospherecomponent (Variables|/Script/Engine.SkyAtmosphere|GetSkyAtmosphereComponent _skyatmosphere))
  (bind _lightcomponent (Variables|/Script/Engine.Light|GetLightComponent _light))
  ;[0.15 0.15 0.15 0.5] Snow falling event
  (Variables|/Game/ThirdPerson/Blueprints/BP_ThirdPersonCharacter.BP_ThirdPersonCharacter_C|SetFootstepSystem _player "/Game/A_Surface_Footstep/Niagara_FX/ParticleSystems/PSN_SnowLight_Surface.PSN_SnowLight_Surface")
  (Audio|Components|Audio|SetSound (Variables|/Game/ThirdPerson/Blueprints/BP_ThirdPersonCharacter.BP_ThirdPersonCharacter_C|GetAudioComponent _player) "/Game/Sounds/SnowStepSound.SnowStepSound")
  (Rendering|SetActorHiddenInGame false)
  (Variables|Default|SetIsSnowing true)
  (if (Variables|/Game/Blueprints/BP_DayNightCycle.BP_DayNightCycle_C|GetIsNight (Variables|Default|GetDayCycle))
    (Development|PrintString "Snow falling is not compatible with night.")
    (else
      (Rendering|Components|Light|SetIntensity _lightcomponent 1.0)
      (Class|LightComponent|SetTemperature _lightcomponent 1.2e+04)
      (Rendering|Components|Light|SetLightColor _lightcomponent "(R=4.654110,G=20.015879,B=42.942680,A=1.000000)" true)
      (Class|SkyAtmosphereComponent|SetRayleighScatteringScale _skyatmospherecomponent 3.0)
      (Class|SkyAtmosphereComponent|SetMieScatteringScale _skyatmospherecomponent 5.0)
      (Class|SkyAtmosphereComponent|SetMieAbsorptionScale _skyatmospherecomponent 0.2)
      (Class|ExponentialHeightFogComponent|SetFogInscatteringColor _component "(R=0.059105,G=0.081315,B=0.810764,A=1.000000)")
      (Class|ExponentialHeightFogComponent|SetFogDensity _component 3e-05)
      (Components|Activation|Activate (Variables|/Script/Engine.Actor|GetRootComponent (Variables|Default|GetSNowNiagara)) false)
      (Class|LandscapeProxy|SetLandscapeMaterialScalarParameterValue _floor "Ice_Amount_Factor" 0.5)
      (Rendering|Material|SetScalarParameterValue (stale EventBeginPlay _returnvalue_2) "Snow_Amount" 0.0 :!class /Script/Engine.MaterialInstanceDynamic)
      (Rendering|Material|SetScalarParameterValue (stale EventBeginPlay _returnvalue_2) "Snow_Hardness" 0.0 :!class /Script/Engine.MaterialInstanceDynamic)
      (bind _newtrack_0 (Timeline|Timeline Play)
        (:Update
          (Class|LandscapeProxy|SetLandscapeMaterialScalarParameterValue _floor "Ice_Amount_Factor" _newtrack_0)
          (if (Variables|Default|GetIsSnowing)
            (bind _newtrack_0_2 (Timeline|Timeline_0 Play)
              (:Update
                (Rendering|Material|SetScalarParameterValue (stale EventBeginPlay _returnvalue_2) "Snow_Amount" _newtrack_0_2 :!class /Script/Engine.MaterialInstanceDynamic)
                (if (Variables|Default|GetIsSnowing)
                  (bind _newtrack_0_3 (Timeline|Timeline_1 Play)
                    (:Update
                      (Rendering|Material|SetScalarParameterValue (stale EventBeginPlay _returnvalue_2) "Snow_Hardness" _newtrack_0_3 :!class /Script/Engine.MaterialInstanceDynamic)))
                  (else
                    (Timeline|Timeline_1 Reverse)))))
            (else
              (Timeline|Timeline_0 Reverse))))))))

(event Custom|SnowFont
  (bind _light (Variables|Default|GetLight))
  (bind _skyatmosphere (Variables|Default|GetSkyAtmosphere))
  (bind _fog (Variables|Default|GetFog))
  (bind _player (Variables|Default|GetPlayer))
  (bind _lightcomponent (Variables|/Script/Engine.Light|GetLightComponent _light))
  (bind _skyatmospherecomponent (Variables|/Script/Engine.SkyAtmosphere|GetSkyAtmosphereComponent _skyatmosphere))
  (bind _component (Variables|/Script/Engine.ExponentialHeightFog|GetComponent _fog))
  ;[0.15 0.15 0.15 0.5] Snow fount
  (Utilities|FlowControl|DoOnce false
    (:Completed
      (Variables|Default|SetIsSnowing false)
      (Components|Activation|Deactivate (Variables|/Script/Engine.Actor|GetRootComponent (Variables|Default|GetSNowNiagara)))
      (Rendering|Components|Light|SetIntensity _lightcomponent 3.0)
      (Class|LightComponent|SetTemperature _lightcomponent 6.5e+03)
      (Rendering|Components|Light|SetLightColor _lightcomponent "(R=1.000000,G=1.000000,B=1.000000,A=1.000000)" true)
      (Class|SkyAtmosphereComponent|SetRayleighScatteringScale _skyatmospherecomponent 0.0331)
      (Class|SkyAtmosphereComponent|SetMieScatteringScale _skyatmospherecomponent 0.003996)
      (Class|SkyAtmosphereComponent|SetMieAbsorptionScale _skyatmospherecomponent 0.000444)
      (Class|ExponentialHeightFogComponent|SetFogInscatteringColor _component "(R=0.000000,G=0.000000,B=0.000000,A=1.000000)")
      (Class|ExponentialHeightFogComponent|SetFogDensity _component 0.0436)
      (Variables|/Game/ThirdPerson/Blueprints/BP_ThirdPersonCharacter.BP_ThirdPersonCharacter_C|SetFootstepSystem _player "/Game/A_Surface_Footstep/Niagara_FX/ParticleSystems/PSN_Dirt_Surface.PSN_Dirt_Surface")
      (Audio|Components|Audio|SetSound (Variables|/Game/ThirdPerson/Blueprints/BP_ThirdPersonCharacter.BP_ThirdPersonCharacter_C|GetAudioComponent _player) "/Game/Sounds/BasicStepSound.BasicStepSound")
      ;[0.15 0.15 0.15 0.5] Snow falling event
      (bind _newtrack_0 (Timeline|Timeline Reverse)
        (:Update
          (Class|LandscapeProxy|SetLandscapeMaterialScalarParameterValue (Variables|Default|GetFloor) "Ice_Amount_Factor" _newtrack_0)
          (if (Variables|Default|GetIsSnowing)
            (bind _newtrack_0_2 (Timeline|Timeline_0 Play)
              (:Update
                (Rendering|Material|SetScalarParameterValue (stale EventBeginPlay _returnvalue_2) "Snow_Amount" _newtrack_0_2 :!class /Script/Engine.MaterialInstanceDynamic)
                (if (Variables|Default|GetIsSnowing)
                  (bind _newtrack_0_3 (Timeline|Timeline_1 Play)
                    (:Update
                      (Rendering|Material|SetScalarParameterValue (stale EventBeginPlay _returnvalue_2) "Snow_Hardness" _newtrack_0_3 :!class /Script/Engine.MaterialInstanceDynamic)))
                  (else
                    (Timeline|Timeline_1 Reverse)))))
            (else
              (Timeline|Timeline_0 Reverse))))))))

(event Custom|SnowEvent
  ;[0.15 0.15 0.15 0.5] Snow Event
  (if (Variables|Default|GetIsSnowing)
    (CallFunction|SnowFont)
    (else
      (CallFunction|ResetFont)
      (CallFunction|SnowFall))))

(event Custom|ResetFont
  (bind _light (Variables|Default|GetLight))
  (bind _skyatmosphere (Variables|Default|GetSkyAtmosphere))
  (bind _fog (Variables|Default|GetFog))
  (bind _player (Variables|Default|GetPlayer))
  (bind _lightcomponent (Variables|/Script/Engine.Light|GetLightComponent _light))
  (bind _skyatmospherecomponent (Variables|/Script/Engine.SkyAtmosphere|GetSkyAtmosphereComponent _skyatmosphere))
  (bind _component (Variables|/Script/Engine.ExponentialHeightFog|GetComponent _fog))
  ;[0.15 0.15 0.15 0.5] Snow fount
  (Utilities|FlowControl|DoOnce false) ; enters at Reset
)

(event EventBeginPlay
  ;[0.15 0.15 0.15 0.5] Snow falling event
  (bind _returnvalue (Actor|GetActorOfClass "/Game/ThirdPerson/Blueprints/BP_ThirdPersonCharacter.BP_ThirdPersonCharacter_C"))
  (Variables|Default|SetPlayer _returnvalue)
  (bind _returnvalue_2 (Rendering|Material|CreateDynamicMaterialInstance (Variables|/Script/Engine.StaticMeshActor|GetStaticMeshComponent (Variables|Default|GetHouse)) 0 "/Game/Materials/Instance/MI_House.MI_House" "None" :!class /Script/Engine.PrimitiveComponent)))

(fn ConstructionScript)