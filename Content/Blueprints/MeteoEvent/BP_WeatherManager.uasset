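; Weather manager that exposes events to trigger tornado, cloud, sandstorm, snow and rain effects in the level.
; On BeginPlay it finds the snow, storm spawner, sandstorm and weather actors by class and forwards each event to them.
; Cloud, snow and rain disable sand effects, while sandstorm toggles on the player's dust plane visibility, calls into snow and rain, and swaps footstep particles and sounds.
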(event Custom|LaunchTornado
  ;[0.15 0.15 0.15 0.5] Launch Tornado
  (Default|StormSpawn (Variables|Default|GetBpStorm)))

(event Custom|CloudEvent
  ;[0.15 0.15 0.15 0.5] Cloud Event
  (Default|Start/StopCloud (Variables|Default|GetBPRain))
  (CallFunction|DisableSandEvent))

(event Custom|SandStormEvent
  (bind _player (Variables|Default|GetPlayer))
  (bind _player_2 (Variables|Default|GetPlayer))
  (bind _player_3 (Variables|Default|GetPlayer))
  (bind _bprain (Variables|Default|GetBPRain))
  (bind _dust_plane (Variables|/Game/ThirdPerson/Blueprints/BP_ThirdPersonCharacter.BP_ThirdPersonCharacter_C|GetDust%20Plane _player_2))
  ;[0.15 0.15 0.15 0.5] Sand storm event
  (if (Rendering|IsVisible _dust_plane)
    (CallFunction|DisableSandEvent)
    (Variables|/Game/ThirdPerson/Blueprints/BP_ThirdPersonCharacter.BP_ThirdPersonCharacter_C|SetFootstepSystem _player_3 "/Game/A_Surface_Footstep/Niagara_FX/ParticleSystems/PSN_Dirt_Surface.PSN_Dirt_Surface")
    (Audio|Components|Audio|SetSound (Variables|/Game/ThirdPerson/Blueprints/BP_ThirdPersonCharacter.BP_ThirdPersonCharacter_C|GetAudioComponent _player_3) "/Game/Sounds/BasicStepSound.BasicStepSound")
    (else
      (Rendering|SetVisibility _dust_plane true false)
      (Default|SnowFont (Variables|Default|GetBpSnow))
      (Default|SandStormEvent (Variables|Default|GetBpSand))
      (Variables|/Game/Weather/BP_Weather.BP_Weather_C|SetIsRainning _bprain true)
      (Default|Start/StopRain _bprain)
      (Variables|/Game/ThirdPerson/Blueprints/BP_ThirdPersonCharacter.BP_ThirdPersonCharacter_C|SetFootstepSystem _player "/Game/A_Surface_Footstep/Niagara_FX/ParticleSystems/PSN_Sand_Surface.PSN_Sand_Surface")
      (Audio|Components|Audio|SetSound (Variables|/Game/ThirdPerson/Blueprints/BP_ThirdPersonCharacter.BP_ThirdPersonCharacter_C|GetAudioComponent _player) "/Game/Sounds/SandStepSound.SandStepSound"))))

(event Custom|Disable%20Sand%20Event
  ;[0.15 0.15 0.15 0.5] Disable Sand
  (Rendering|SetVisibility (Variables|/Game/ThirdPerson/Blueprints/BP_ThirdPersonCharacter.BP_ThirdPersonCharacter_C|GetDust%20Plane (Variables|Default|GetPlayer)) false false)
  (Default|DisableSand (Variables|Default|GetBpSand)))

(event Custom|Snow%20Event
  ;[0.15 0.15 0.15 0.5] Snow event
  (Default|SnowEvent (Variables|Default|GetBpSnow))
  (CallFunction|DisableSandEvent))

(event Custom|Rain%20Event
  ;[0.15 0.15 0.15 0.5] Rain event
  (Default|SnowFont (Variables|Default|GetBpSnow))
  (CallFunction|DisableSandEvent)
  (Default|Start/StopRain (Variables|Default|GetBPRain)))

(event EventBeginPlay
  (bind _returnvalue (Actor|GetActorOfClass "/Game/Blueprints/MeteoEvent/BP_SnowEvent.BP_SnowEvent_C"))
  (Variables|Default|SetBpSnow _returnvalue)
  (bind _returnvalue_2 (Actor|GetActorOfClass "/Game/Blueprints/MeteoEvent/BP_StormSpawner.BP_StormSpawner_C"))
  (Variables|Default|SetBpStorm _returnvalue_2)
  (bind _returnvalue_3 (Actor|GetActorOfClass "/Game/Blueprints/MeteoEvent/BP_SandStorm.BP_SandStorm_C"))
  (Variables|Default|SetBpSand _returnvalue_3)
  (bind _returnvalue_4 (Actor|GetActorOfClass "/Game/Weather/BP_Weather.BP_Weather_C"))
  (Variables|Default|SetBPRain _returnvalue_4))

(fn ConstructionScript)