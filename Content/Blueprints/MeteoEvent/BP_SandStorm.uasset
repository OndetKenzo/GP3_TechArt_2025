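; Sandstorm weather event Blueprint that toggles the scene's atmosphere between storm and clear looks through two events.
; SandStormEvent hides the Fogs actors, tints the light orange, changes fog color and density, raises Rayleigh scattering and applies a distortion post-process material.
; DisableSand shows those actors again, sets hard-coded clear values and empties the blendables, leaving indirect lighting intensity unrestored.
; Both events apply every change inside the Fogs loop.
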(event Custom|SandStormEvent
  (bind _light (Variables|Default|GetLight))
  (bind _fog (Variables|Default|GetFog))
  (bind _component (Variables|/Script/Engine.ExponentialHeightFog|GetComponent _fog))
  (bind _lightcomponent (Variables|/Script/Engine.Light|GetLightComponent _light))
  (for _array_element (Variables|Default|GetFogs)
    (Rendering|SetActorHiddenInGame _array_element true)
    (Rendering|Components|Light|SetLightColor _lightcomponent "(R=0.687500,G=0.379070,B=0.172445,A=1.000000)" true)
    (Class|LightComponent|SetIndirectLightingIntensity _lightcomponent 0.5)
    (Class|ExponentialHeightFogComponent|SetFogDensity _component 0.02)
    (Class|ExponentialHeightFogComponent|SetFogInscatteringColor _component "(R=1.000000,G=0.986423,B=0.302083,A=1.000000)")
    (Utilities|Struct|SetmembersinPostProcessSettings (Variables|/Script/Engine.PostProcessVolume|GetSettings (Variables|Default|GetPostProcessVolume)) (Utilities|Struct|MakeWeightedBlendables (Utilities|Array|MakeArray (Utilities|Struct|MakeWeightedBlendable 1.0 (Variables|Default|GetMaterialDIstorsion)))))
    (Class|SkyAtmosphereComponent|SetRayleighScatteringScale (Variables|/Script/Engine.SkyAtmosphere|GetSkyAtmosphereComponent (Variables|Default|GetSkyAtmosphere)) 0.2)))

(event Custom|DisableSand
  (bind _fog (Variables|Default|GetFog))
  (bind _component (Variables|/Script/Engine.ExponentialHeightFog|GetComponent _fog))
  (for _array_element (Variables|Default|GetFogs)
    (Rendering|SetActorHiddenInGame _array_element false)
    (Rendering|Components|Light|SetLightColor (Variables|/Script/Engine.Light|GetLightComponent (Variables|Default|GetLight)) "(R=1.000000,G=1.000000,B=1.000000,A=1.000000)" true)
    (Class|ExponentialHeightFogComponent|SetFogInscatteringColor _component "(R=0.000000,G=0.000000,B=0.000000,A=1.000000)")
    (Class|ExponentialHeightFogComponent|SetFogDensity _component 0.0436)
    (Utilities|Struct|SetmembersinPostProcessSettings (Variables|/Script/Engine.PostProcessVolume|GetSettings (Variables|Default|GetPostProcessVolume)) (Utilities|Struct|MakeWeightedBlendables 0))
    (Class|SkyAtmosphereComponent|SetRayleighScatteringScale (Variables|/Script/Engine.SkyAtmosphere|GetSkyAtmosphereComponent (Variables|Default|GetSkyAtmosphere)) 0.042418)))

(fn ConstructionScript)