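; BP_StormSpawner spawns a temporary storm weather effect around the player.
; Its StormSpawn event spawns the NS_Storm Niagara system just below player character 0, then destroys it after a fixed delay.
; A StormCount guard allows only one storm at a time and prints a limit message when another is requested.
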(event Custom|StormSpawn
  (if (< (Variables|Default|GetStormCount) 1)
    (bind _returnvalue (Niagara|SpawnSystematLocation "/Game/VFX/System/NS_Storm.NS_Storm" (- (Transformation|GetActorLocation (Game|GetPlayerCharacter 0)) "0.000000,0.000000,300.000000")))
    (Variables|Default|SetStormCount (+ (Variables|Default|GetStormCount) 1))
    (Utilities|FlowControl|Delay 25.0)
    (Components|DestroyComponent _returnvalue)
    (Variables|Default|SetStormCount (- (Variables|Default|GetStormCount) 1))
    (else
      (Development|PrintString "You reached the storm limit."))))

(fn ConstructionScript)