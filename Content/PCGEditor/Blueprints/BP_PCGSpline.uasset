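; Editable spline actor that drives a PCG component to scatter content such as forest, rocks, houses, flowers or barriers.
; It spawns BP_SplineWayPoint actors as point handles, keeping their indices in sync through moves, inserts and deletes.
; Point edits regenerate PCG with a random seed and turn waypoints toward the spline centroid.
; ChangePCGType picks area graphs for closed loops or Line variants for open splines, and adds actor tags.
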(event EventBeginPlay)

(event Collision|EventActorBeginOverlap
  (params (OtherActor :type Actor%20Object%20Reference)))

(event EventTick
  (params (DeltaSeconds :type Float%20%28single-precision%29)))

(fn ConstructionScript)

(fn AddSplinePoints
  (params (WayPointPos :type Vector))
  (Spline|AddSplinePoint (Variables|Default|GetSpline) WayPointPos "World" true))

(fn IsLooping
  (params (value :type Boolean))
  (Spline|SetClosedLoop (Variables|Default|GetSpline) value true)
  (if (not value)
    (Class|PCGComponent|SetGraph (Variables|Default|GetPCG) "/Game/PCGEditor/PCG/PCG_SplineTesterLine.PCG_SplineTesterLine")))

(fn SpawnWayPointMesh
  (params (MeshPosition :type Vector) (SplineIndex :type Integer))
  (bind _returnvalue (Game|SpawnActorfromClass "/Game/PCGEditor/Blueprints/BP_SplineWayPoint.BP_SplineWayPoint_C" (Math|Transform|MakeTransform MeshPosition "0, 0, 0" "1.000000,1.000000,1.000000") "Undefined" "MultiplyWithRoot" 0 0))
  (bind _returnvalue_2 (Utilities|Array|Add (Variables|Default|GetMeshArray) _returnvalue))
  (Variables|/Game/PCGEditor/Blueprints/BP_SplineWayPoint.BP_SplineWayPoint_C|SetWayPointIndex _returnvalue _returnvalue_2)
  (Variables|/Game/PCGEditor/Blueprints/BP_SplineWayPoint.BP_SplineWayPoint_C|SetSplineIndex _returnvalue SplineIndex))

(fn SpawnSplineWayPoints
  (params (SplineIndex :type Integer))
  (bind _spline (Variables|Default|GetSpline))
  (for _index (range 0 (- (Spline|GetNumberOfSplinePoints _spline) 1))
    (CallFunction|SpawnWayPointMesh (.position (Spline|GetSplinePointAt _spline _index "World")) SplineIndex))
  (CallFunction|RegeneratePCG)
  (CallFunction|UpdateCentroid))

(fn SetWayPointPosition
  (params (WayPointIndex :type Integer) (New%20Position :type Vector))
  (Spline|SetLocationatSplinePoint (Variables|Default|GetSpline) WayPointIndex New%20Position "World" true)
  (CallFunction|RegeneratePCG)
  (CallFunction|UpdateCentroid))

(fn DeleteSplinePoint
  (params (index :type Integer))
  (bind _mesharray (Variables|Default|GetMeshArray))
  (Spline|RemoveSplinePoint (Variables|Default|GetSpline) index true)
  (Actor|DestroyActor (Utilities|Array|Get(acopy) _mesharray index))
  (Utilities|Array|RemoveIndex _mesharray index)
  (CallFunction|RegeneratePCG)
  (CallFunction|UpdateIndexesValues index true)
  (CallFunction|UpdateCentroid))

(fn RegeneratePCG
  (bind _pcg (Variables|Default|GetPCG))
  (Variables|/Script/PCG.PCGComponent|SetSeed _pcg (Math|Random|RandomInteger 15000))
  (Class|PCGComponent|Cleanup _pcg false)
  (PCG|Generate _pcg false))

(fn UpdateIndexesValues
  (params (Index :type Integer) (isADeleteIndex :type Boolean))
  (for (_array_element _array_index) (Variables|Default|GetMeshArray)
    (if isADeleteIndex
      (if (>= _array_index Index)
        (Variables|/Game/PCGEditor/Blueprints/BP_SplineWayPoint.BP_SplineWayPoint_C|SetWayPointIndex _array_element (- (Variables|/Game/PCGEditor/Blueprints/BP_SplineWayPoint.BP_SplineWayPoint_C|GetWayPointIndex _array_element) 1)))
      (elif (>= _array_index Index)
        (Variables|/Game/PCGEditor/Blueprints/BP_SplineWayPoint.BP_SplineWayPoint_C|SetWayPointIndex _array_element (+ (Variables|/Game/PCGEditor/Blueprints/BP_SplineWayPoint.BP_SplineWayPoint_C|GetWayPointIndex _array_element) 1))))))

(fn DestroySpline
  (for _array_element (Variables|Default|GetMeshArray)
    (Actor|DestroyActor _array_element))
  (Actor|DestroyActor))

(fn GetWayPointCount
  (return (Spline|GetNumberOfSplinePoints (Variables|Default|GetSpline))))

(fn AddWayPointtoSpecificIndex
  (params (Index :type Integer))
  (bind _mesharray (Variables|Default|GetMeshArray))
  (bind _output (Utilities|Array|Get(acopy) _mesharray Index))
  (bind _returnvalue (Transformation|GetActorLocation _output))
  (bind _returnvalue_2 (Transformation|GetActorRightVector _output))
  (bind _returnvalue_3 (* 1e+02 _returnvalue_2))
  (bind _returnvalue_4 (+ _returnvalue _returnvalue_3))
  (Spline|AddSplinePointatIndex (Variables|Default|GetSpline) _returnvalue_4 Index "World" true)
  (bind _returnvalue_5 (Game|SpawnActorfromClass "/Game/PCGEditor/Blueprints/BP_SplineWayPoint.BP_SplineWayPoint_C" (Math|Transform|MakeTransform _returnvalue_4 "0, 0, 0" "1.000000,1.000000,1.000000") "Undefined" "MultiplyWithRoot" 0 0))
  (Variables|/Game/PCGEditor/Blueprints/BP_SplineWayPoint.BP_SplineWayPoint_C|SetSplineIndex _returnvalue_5 (Variables|/Game/PCGEditor/Blueprints/BP_SplineWayPoint.BP_SplineWayPoint_C|GetSplineIndex _output))
  (CallFunction|UpdateMeshArrayAfterAnAdd Index _returnvalue_5)
  (CallFunction|RegeneratePCG)
  (CallFunction|UpdateCentroid))

(fn UpdateMeshArrayAfterAnAdd
  (params (Index :type Integer) (toAdd :type BP%20Spline%20Way%20Point%20Object%20Reference))
  (bind _newarray (LocalVariables|GetNewArray))
  (for (_array_element _array_index) (Variables|Default|GetMeshArray)
    (if (== _array_index Index)
      (bind _returnvalue (Utilities|Array|Add _newarray toAdd))
      (Variables|/Game/PCGEditor/Blueprints/BP_SplineWayPoint.BP_SplineWayPoint_C|SetWayPointIndex toAdd _returnvalue))
    (bind _returnvalue_2 (Utilities|Array|Add _newarray _array_element))
    (Variables|/Game/PCGEditor/Blueprints/BP_SplineWayPoint.BP_SplineWayPoint_C|SetWayPointIndex _array_element _returnvalue_2))
  (Variables|Default|SetMeshArray (LocalVariables|GetNewArray)))

(fn ChangePCGType
  (params (Type :type EPCGType%20Enum :default "NewEnumerator0"))
  (bind _tagarray (LocalVariables|GetTagArray))
  (bind _tagarray_2 (LocalVariables|GetTagArray))
  (bind _pcg (Variables|Default|GetPCG))
  (bind _pcg_2 (Variables|Default|GetPCG))
  (bind _tagarray_3 (LocalVariables|GetTagArray))
  (bind _tagarray_4 (LocalVariables|GetTagArray))
  (bind _tagarray_5 (LocalVariables|GetTagArray))
  (bind _tagarray_6 (LocalVariables|GetTagArray))
  (bind _tagarray_7 (LocalVariables|GetTagArray))
  (if (Class|SplineComponent|IsClosedLoop (Variables|Default|GetSpline))
    (switch Utilities|FlowControl|Switch|SwitchonEPCGType Type
      (:NewEnumerator0
        (Class|PCGComponent|SetGraph _pcg_2 "/Game/PCGEditor/PCG/PCG_Forest.PCG_Forest")
        (Utilities|Array|Add _tagarray_3 "PCG_Forest")
        (Variables|Default|SetTags _tagarray_3))
      (:NewEnumerator1
        (Class|PCGComponent|SetGraph _pcg_2 "/Game/PCGEditor/PCG/PCG_Rocks.PCG_Rocks")
        (Utilities|Array|Add _tagarray_7 "PCG_Rocks")
        (Variables|Default|SetTags _tagarray_7))
      (:NewEnumerator3
        (Class|PCGComponent|SetGraph _pcg_2 "/Game/PCGEditor/PCG/PCG_Houses.PCG_Houses")
        (Utilities|Array|Add _tagarray "PCG_Houses")
        (Variables|Default|SetTags _tagarray))
      (:NewEnumerator4
        (Class|PCGComponent|SetGraph _pcg_2 "/Game/PCGEditor/PCG/PCG_Flowers.PCG_Flowers")
        (Utilities|Array|Add _tagarray_5 "PCG_Flowers")
        (Variables|Default|SetTags _tagarray_5))
      (:NewEnumerator5
        (Class|PCGComponent|SetGraph _pcg_2 "/Game/PCGEditor/PCG/PCG_AnimalRocks.PCG_AnimalRocks")
        (Utilities|Array|Add _tagarray_6 "PCG_AnimalRocks")
        (Variables|Default|SetTags _tagarray_6))
      (:NewEnumerator6
        (Class|PCGComponent|SetGraph _pcg_2 "/Game/PCGEditor/PCG/PCG_Barrier.PCG_Barrier")
        (Utilities|Array|Add _tagarray_2 "PCG_Barrier")
        (Variables|Default|SetTags _tagarray_2)))
    (CallFunction|RegeneratePCG)
    (else
      (switch Utilities|FlowControl|Switch|SwitchonEPCGType Type
        (:NewEnumerator0
          (Class|PCGComponent|SetGraph _pcg "/Game/PCGEditor/PCG/PCG_ForestLine.PCG_ForestLine"))
        (:NewEnumerator1
          (Class|PCGComponent|SetGraph _pcg "/Game/PCGEditor/PCG/PCG_RocksLine.PCG_RocksLine"))
        (:NewEnumerator3
          (Class|PCGComponent|SetGraph _pcg "/Game/PCGEditor/PCG/PCG_HousesLine.PCG_HousesLine"))
        (:NewEnumerator4
          (Class|PCGComponent|SetGraph _pcg "/Game/PCGEditor/PCG/PCG_FlowersLine.PCG_FlowersLine"))
        (:NewEnumerator5
          (Class|PCGComponent|SetGraph _pcg "/Game/PCGEditor/PCG/PCG_AnimalRocksLine.PCG_AnimalRocksLine"))
        (:NewEnumerator6
          (Class|PCGComponent|SetGraph _pcg "/Game/PCGEditor/PCG/PCG_BarrierLine.PCG_BarrierLine")))
      (Utilities|Array|Add _tagarray_4 "PCG_Barrier")
      (Variables|Default|SetTags _tagarray_4)
      (CallFunction|RegeneratePCG))))

(fn UpdateCentroid
  (bind _spline (Variables|Default|GetSpline))
  (bind _returnvalue (Spline|GetNumberOfSplinePoints _spline))
  (Variables|Default|SetCentroid "0, 0, 0")
  (for _index (range 0 (- _returnvalue 1))
    (Variables|Default|SetCentroid (+ (Variables|Default|GetCentroid) (.position (Spline|GetSplinePointAt _spline _index "World")))))
  (bind _output_get (Variables|Default|SetCentroid (/ (Variables|Default|GetCentroid) _returnvalue)))
  (for _array_element (Variables|Default|GetMeshArray)
    (Transformation|SetActorRotation _array_element (Math|Rotator|FindLookatRotation (Transformation|GetActorLocation _array_element) _output_get))))